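; BP_Tunnel is a tunnel segment for an endless obstacle run, with a random color and a rotating holed wall.
; Its construction script picks the color material, RandomizeWall sets a random hole mesh and roll, and Tick keeps the wall spinning.
; When the player overlaps TriggerZone, it has TunnelSpawner add a new segment and destroys itself.
; A player hit on the wall marks BP_Player dead and displays the restart option.
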(event OnComponentBeginOverlap(TriggerZone)
  (params (OverlappedComponent :type Primitive%20Component%20Object%20Reference) (OtherActor :type Actor%20Object%20Reference) (OtherComp :type Primitive%20Component%20Object%20Reference) (OtherBodyIndex :type Integer) (bFromSweep :type Boolean) (SweepResult :type Hit%20Result%20Structure%20%28by%20ref%29))
  ;[1 1 1] "Refreshing" amount of tunnels by deleting previous and adding new ones
  (Utilities|Casting|CastToBP_Player OtherActor)
  (Default|SpawnTunnelatSpawnPoint (Variables|Default|GetTunnelSpawner))
  (Actor|DestroyActor))

(event OnComponentHit(WallMesh)
  (params (HitComponent :type Primitive%20Component%20Object%20Reference) (OtherActor :type Actor%20Object%20Reference) (OtherComp :type Primitive%20Component%20Object%20Reference) (NormalImpulse :type Vector :default "0, 0, 0") (Hit :type Hit%20Result%20Structure%20%28by%20ref%29))
  ;[1 1 1] Setting ability to restart game after hitting the wall
  (bind _asbp_player (Utilities|Casting|CastToBP_Player OtherActor))
  (Variables|/Game/InfiniteMatrix/Blueprints/BP_Player.BP_Player_C|SetIsDead _asbp_player true)
  (Default|DisplayRestart _asbp_player))

(event EventBeginPlay)

(event EventTick
  (params (DeltaSeconds :type Float%20%28single-precision%29))
  ;[1 1 1] Adding rotation to the walls inside the tunnels
  (Transformation|AddLocalRotation (Variables|Default|GetWallMesh) (Math|Rotator|MakeRotator (* DeltaSeconds (Variables|Default|GetRotateSpeed)) 0.0 0.0) false false))

(fn ConstructionScript
  ;[1 1 1] Setting random materials to create variously colored tunnels!
  (Rendering|Material|SetMaterial (Variables|Debug|GetStaticMeshComponent) 0 (Utilities|Select :Index (Math|Random|RandomIntegerinRange 0 3) :Option%200 "/Game/InfiniteMatrix/Materials/TunnelMaterials/MI_TunnelBlue.MI_TunnelBlue" :Option%201 "/Game/InfiniteMatrix/Materials/TunnelMaterials/MI_TunnelGreen.MI_TunnelGreen" :Option%202 "/Game/InfiniteMatrix/Materials/TunnelMaterials/MI_TunnelRed.MI_TunnelRed" :Option%203 "/Game/InfiniteMatrix/Materials/TunnelMaterials/MI_TunnelPurple.MI_TunnelPurple")))

(fn RandomizeWall
  (Components|StaticMesh|SetStaticMesh (Variables|Default|GetWallMesh) (Utilities|Select :Index (Math|Random|RandomIntegerinRange 0 19) :Option%200 "/Game/InfiniteMatrix/Meshes/WallMeshes/SM_Hole_010.SM_Hole_010" :Option%201 "/Game/InfiniteMatrix/Meshes/WallMeshes/SM_Hole_011.SM_Hole_011" :Option%202 "/Game/InfiniteMatrix/Meshes/WallMeshes/SM_Hole_012.SM_Hole_012" :Option%203 "/Game/InfiniteMatrix/Meshes/WallMeshes/SM_Hole_013.SM_Hole_013" :Option%204 "/Game/InfiniteMatrix/Meshes/WallMeshes/SM_Hole_020.SM_Hole_020" :Option%205 "/Game/InfiniteMatrix/Meshes/WallMeshes/SM_Hole_021.SM_Hole_021" :Option%206 "/Game/InfiniteMatrix/Meshes/WallMeshes/SM_Hole_022.SM_Hole_022" :Option%207 "/Game/InfiniteMatrix/Meshes/WallMeshes/SM_Hole_023.SM_Hole_023" :Option%208 "/Game/InfiniteMatrix/Meshes/WallMeshes/SM_Hole_030.SM_Hole_030" :Option%209 "/Game/InfiniteMatrix/Meshes/WallMeshes/SM_Hole_031.SM_Hole_031" :Option%2010 "/Game/InfiniteMatrix/Meshes/WallMeshes/SM_Hole_032.SM_Hole_032" :Option%2011 "/Game/InfiniteMatrix/Meshes/WallMeshes/SM_Hole_033.SM_Hole_033" :Option%2012 "/Game/InfiniteMatrix/Meshes/WallMeshes/SM_Hole_040.SM_Hole_040" :Option%2013 "/Game/InfiniteMatrix/Meshes/WallMeshes/SM_Hole_041.SM_Hole_041" :Option%2014 "/Game/InfiniteMatrix/Meshes/WallMeshes/SM_Hole_042.SM_Hole_042" :Option%2015 "/Game/InfiniteMatrix/Meshes/WallMeshes/SM_Hole_043.SM_Hole_043" :Option%2016 "/Game/InfiniteMatrix/Meshes/WallMeshes/SM_Hole050.SM_Hole050" :Option%2017 "/Game/InfiniteMatrix/Meshes/WallMeshes/SM_Hole0511.SM_Hole0511" :Option%2018 "/Game/InfiniteMatrix/Meshes/WallMeshes/SM_Hole0521.SM_Hole0521" :Option%2019 "/Game/InfiniteMatrix/Meshes/WallMeshes/SM_Hole0531.SM_Hole0531"))
  (Transformation|AddLocalRotation (Variables|Default|GetWallMesh) (Math|Rotator|MakeRotator (Math|Random|RandomFloatinRange 0.0 3.6e+02) 0.0 0.0) false false))