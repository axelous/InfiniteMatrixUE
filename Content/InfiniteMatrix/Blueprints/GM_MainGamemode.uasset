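; GM_MainGamemode is the game mode Blueprint that sets up the player HUD and times the current flyover.
; BeginPlay creates the HUD widget, stores it in PlayerHUD and adds it to the viewport.
; Tick runs through a one-second Delay, which ignores re-triggers while pending, so PlaytimeSec counts up roughly once per second and rolls over into PlaytimeMin each minute.
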(event EventBeginPlay
  ;[1 1 1] Creating HUD
  (bind _returnvalue (UserInterface|CreateWidget "/Game/InfiniteMatrix/UI/Player_HUD.Player_HUD_C"))
  (bind _output_get (Variables|Default|SetPlayerHUD _returnvalue))
  (UserInterface|Viewport|AddtoViewport _output_get 0))

(event EventTick
  (params (DeltaSeconds :type Float%20%28single-precision%29))
  ;[1 1 1] Creating a timer of current flyover
  (Utilities|FlowControl|Delay 1.0)
  (Variables|Default|SetPlaytimeSec (+ (Variables|Default|GetPlaytimeSec) 1))
  (if (> (Variables|Default|GetPlaytimeSec) 59)
    (Variables|Default|SetPlaytimeMin (+ (Variables|Default|GetPlaytimeMin) 1))
    (Variables|Default|SetPlaytimeSec 0)))

(fn ConstructionScript)